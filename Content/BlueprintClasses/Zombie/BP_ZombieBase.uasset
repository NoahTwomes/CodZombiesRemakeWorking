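; BP_ZombieBase is the base zombie Blueprint, handling attack montages and damage to players.
; MC_AnimMontage plays or stops montages, and a sphere overlap applies damage while CanDamage is set, throttled by a briefly reset DoOnce.
; Hit directly lowers a BP_CharacterBase's Health and calls Die at zero.
; If multiple characters exist, death also disables input, shows the game-over widget and server-travels to Nacht der Untoten after a delay.
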(event OnComponentBeginOverlap(Sphere)
  (params (OverlappedComponent :type Primitive%20Component%20Object%20Reference) (OtherActor :type Actor%20Object%20Reference) (OtherComp :type Primitive%20Component%20Object%20Reference) (OtherBodyIndex :type Integer) (bFromSweep :type Boolean) (SweepResult :type Hit%20Result%20Structure%20%28by%20ref%29))
  (if (Variables|Default|GetcanDamage)
    (Utilities|FlowControl|DoOnce false :!label _label
      (:Completed
        (Game|Damage|ApplyDamage OtherActor 5e+01 0 0)
        (Utilities|FlowControl|Delay 0.0001)
        (goto _label Reset)))))

(event Custom|MC_AnimMontage
  (params (Stop? :type Boolean) (AnimMontage :type Anim%20Montage%20Object%20Reference) (In%20play%20rate :type Float%20%28double-precision%29))
  (if Stop?
    (Animation|StopAnimMontage AnimMontage)
    (else
      (Animation|PlayAnimMontage AnimMontage In%20play%20rate "None"))))

(event Custom|Hit
  (params (Actor :type Actor%20Object%20Reference))
  (bind _asbp_character_base (Utilities|Casting|CastToBP_CharacterBase Actor))
  (bind _output_get (Variables|/Script/CodZombiesRemake.CharacterBase|SetHealth _asbp_character_base (- (Variables|/Script/CodZombiesRemake.CharacterBase|GetHealth _asbp_character_base) 25.0)))
  (if (<= _output_get 0.0)
    (Class|CharacterBase|Die _asbp_character_base)
    (bind _outactors (Actor|GetAllActorsOfClass "/Game/BlueprintClasses/Player/BP_CharacterBase.BP_CharacterBase_C"))
    (if (> (Utilities|Array|Length _outactors) 1)
      (Input|DisableInput _asbp_character_base 0)
      (bind _returnvalue (UserInterface|CreateWidget "/Game/BlueprintClasses/Player/HUD/W_GameOverScreen.W_GameOverScreen_C" (Game|GetPlayerController 0)))
      (UserInterface|Viewport|AddtoViewport _returnvalue 0)
      (Utilities|FlowControl|Delay 5.0)
      (Development|ExecuteConsoleCommand "ServerTravel map_Nacht_der_Untoten" 0))))

(event EventBeginPlay)

(event Collision|EventActorBeginOverlap
  (params (OtherActor :type Actor%20Object%20Reference)))

(event EventTick
  (params (DeltaSeconds :type Float%20%28single-precision%29)))

(fn ConstructionScript)