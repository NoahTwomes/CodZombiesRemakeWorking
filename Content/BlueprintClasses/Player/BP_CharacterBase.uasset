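; Player character base for a zombies mode, handling sprint, damage, health regeneration, downing, revival and game over.
; Sprint, damage and revive input relay through server/client-named events; zero health stops movement and decrements the GameMode's PlayersAlive.
; Reviving messages an overlapping character via InteractInterface, increments that count and clears the caller's own IsDead.
; Tick refills health after delays and, on authority with nobody alive, triggers game over and ServerTravel to Nacht der Untoten.
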(event Custom|DamageOnClient
  (params (Damage :type Float%20%28double-precision%29))
  (bind _output_get (Variables|Default|SetHealth (Math|Float|Clamp(Float) (- (Variables|Default|GetHealth) Damage) 0.0 (Variables|Default|GetMaxHealth))))
  (if (== _output_get 0.0)
    (Variables|/Script/Engine.CharacterMovementComponent|SetMaxWalkSpeed (Variables|Character|GetCharacterMovement) 0.0)
    (Utilities|FlowControl|DoOnce false
      (:Completed
        (CallFunction|AddDeadPlayers)
        (Variables|Default|SetIsDead true)))))

(event Custom|DamageOnServer
  (params (Damage :type Float%20%28double-precision%29))
  (CallFunction|DamageonClient Damage))

(event Custom|Clnt_Walk
  (Class|CharacterBase|Walk))

(event Custom|Srv_Walk
  (CallFunction|ClntWalk))

(event Custom|AddDeadPlayers
  (params (NewParam :type Zombies%20Game%20Mode%20Object%20Reference))
  (bind _as_zombies_game_mode (Variables|Default|GetAs%20Zombies%20Game%20Mode))
  (Variables|/Script/CodZombiesRemake.ZombiesGameMode|SetPlayersAlive _as_zombies_game_mode (- (Variables|/Script/CodZombiesRemake.ZombiesGameMode|GetPlayersAlive _as_zombies_game_mode) 1)))

(event Custom|ReviveClient
  (bind _as_zombies_game_mode (Variables|Default|GetAs%20Zombies%20Game%20Mode))
  (bind _array_element (Utilities|Array|ForEachLoopwithBreak (Collision|GetOverlappingActors "BP_CharacterBase_C" :!class /Script/Engine.Actor) :!label _label)
    (:LoopBody
      (if (Utilities|DoesObjectImplementInterface _array_element "/Game/BlueprintClasses/Player/InteractInterface.InteractInterface_C")
        (Class|InteractInterface|NewFunction(Message) _array_element)
        (Utilities|FlowControl|Sequence
          (:then_0
            (goto _label Break))
          (:then_1
            (Variables|Default|SetIsDead false)
            (Variables|/Script/CodZombiesRemake.ZombiesGameMode|SetPlayersAlive _as_zombies_game_mode (+ (Variables|/Script/CodZombiesRemake.ZombiesGameMode|GetPlayersAlive _as_zombies_game_mode) 1))))))))

(event Custom|ReviveServer
  (CallFunction|ReviveClient))

(event Custom|Clnt_Sprint
  (Class|CharacterBase|Sprint))

(event Custom|Srv_Sprint
  (CallFunction|ClntSprint))

(event Custom|AddDeadPlayerssrv
  (CallFunction|AddDeadPlayers))

(event Custom|GameOver
  (bind _returnvalue (UserInterface|CreateWidget "/Game/BlueprintClasses/Player/HUD/W_GameOverScreen.W_GameOverScreen_C"))
  (UserInterface|Viewport|AddtoViewport _returnvalue 0))

(event Custom|GameOverSrv
  (CallFunction|GameOver)
  (Utilities|FlowControl|Delay 5.0)
  (Development|ExecuteConsoleCommand "ServerTravel map_Nacht_der_Untoten" 0))

(event EventNewFunction
  (Variables|/Script/Engine.CharacterMovementComponent|SetMaxWalkSpeed (Variables|Character|GetCharacterMovement) 6e+02)
  (Variables|Default|SetMaxHealth 1.5e+02)
  (Variables|Default|SetHealth 1.5e+02)
  (Development|PrintString "Revived")
  (Utilities|FlowControl|DoOnce false) ; enters at Reset
)

(event Collision|EventActorBeginOverlap
  (params (OtherActor :type Actor%20Object%20Reference)))

(event EventTick
  (params (DeltaSeconds :type Float%20%28single-precision%29))
  (Utilities|FlowControl|Sequence
    (:then_0
      (if (not (Variables|Default|GetIsDead))
        (if (>= (Variables|Default|GetHealth) 55.0)
          (Utilities|FlowControl|Delay 5.0)
          (Variables|Default|SetHealth (Variables|Default|GetMaxHealth))
          (else
            (Utilities|FlowControl|Delay 8.0)
            (Variables|Default|SetHealth (Variables|Default|GetMaxHealth))))))
    (:then_1
      (Networking|SwitchHasAuthority
        (:Authority
          (if (== (Variables|/Script/CodZombiesRemake.ZombiesGameMode|GetPlayersAlive (Variables|Default|GetAs%20Zombies%20Game%20Mode)) 0)
            (Utilities|FlowControl|DoOnce false
              (:Completed
                (CallFunction|GameOverSrv)))))))))

(event Game|Damage|EventAnyDamage
  (params (Damage :type Float%20%28single-precision%29) (DamageType :type Damage%20Type%20Object%20Reference) (InstigatedBy :type Controller%20Object%20Reference) (DamageCauser :type Actor%20Object%20Reference))
  (CallFunction|DamageonServer Damage))

(event EventBeginPlay
  (bind _aszombies_game_mode (Utilities|Casting|CastToZombiesGameMode (Game|GetGameMode)))
  (Variables|Default|SetAs%20Zombies%20Game%20Mode _aszombies_game_mode))

(event Input|KeyboardEvents|E
  (params (Key :type Key%20Structure :default "None"))
  (:Pressed
    (CallFunction|ReviveServer)))

(event Input|KeyboardEvents|LeftShift
  (params (Key :type Key%20Structure :default "None"))
  (:Pressed
    (CallFunction|SrvSprint))
  (:Released
    (CallFunction|SrvWalk)))

(fn ConstructionScript)

(fn OnRepPlayersDead)