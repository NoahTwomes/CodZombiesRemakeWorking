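; Gore effect actor that bursts into four physics gib meshes with a blood spray and sound on spawn.
; BeginPlay gives each gib a random upward impulse and switches its blood trail off after a short delay.
; Spray and trail particle collisions spawn splatter decals with random atlas frame, size and, for spray, lifespan.
; A Hit event starts polling loops that toggle each trail according to its gib's velocity.
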(event Custom|CustomEvent_5
  (params (EventName :type Name) (EmitterTime :type Float%20%28single-precision%29) (ParticleTime :type Integer) (Location :type Vector) (Velocity :type Vector) (Direction :type Vector) (Normal :type Vector) (BoneName :type Name) (PhysMat :type Physical%20Material%20Object%20Reference))
  (bind _returnvalue (Math|Random|RandomFloatinRange 2e+01 5e+01))
  ;[1 1 1] Blood Trails
  (switch int (Math|Random|RandomIntegerinRange 1 2)
    (:1
      (bind _returnvalue_2 (Rendering|Material|CreateDynamicMaterialInstance "/Game/ZombiesAndDemons/BloodEffects/Materials/M_Splatter_decal.M_Splatter_decal" "None" :!class /Script/Engine.KismetMaterialLibrary))
      (Rendering|Material|SetScalarParameterValue _returnvalue_2 "Frame" (Math|Conversions|ToFloat(Integer) (Math|Random|RandomInteger 16)) :!class /Script/Engine.MaterialInstanceDynamic)
      (Rendering|Decal|SpawnDecalatLocation _returnvalue_2 (Math|Vector|MakeVector 1.0 _returnvalue _returnvalue) Location (Math|Conversions|RotationFromXVector (* Normal -1.0)) 2e+01))))

(event Custom|CustomEvent
  (params (EventName :type Name) (EmitterTime :type Float%20%28single-precision%29) (ParticleTime :type Integer) (Location :type Vector) (Velocity :type Vector) (Direction :type Vector) (Normal :type Vector) (BoneName :type Name) (PhysMat :type Physical%20Material%20Object%20Reference))
  (bind _returnvalue (Math|Random|RandomFloatinRange 2e+01 5e+01))
  (bind _returnvalue_2 (* Normal -1.0))
  (bind _returnvalue_3 (Math|Random|RandomFloatinRange 2e+01 5e+01))
  (bind _returnvalue_4 (Math|Conversions|RotationFromXVector _returnvalue_2))
  ;[1 1 1] BloodSplatter
  (bind _returnvalue_5 (Rendering|Material|CreateDynamicMaterialInstance "/Game/ZombiesAndDemons/BloodEffects/Materials/M_Splatter_decal.M_Splatter_decal" "None" :!class /Script/Engine.KismetMaterialLibrary))
  (Rendering|Material|SetScalarParameterValue _returnvalue_5 "Frame" (Math|Conversions|ToFloat(Integer) (Math|Random|RandomInteger 16)) :!class /Script/Engine.MaterialInstanceDynamic)
  (switch int (Math|Random|RandomIntegerinRange 0 10)
    (:Default
      (Rendering|Decal|SpawnDecalatLocation _returnvalue_5 (Math|Vector|MakeVector 1.0 _returnvalue _returnvalue) Location _returnvalue_4 5.0))
    (:0
      (Rendering|Decal|SpawnDecalatLocation _returnvalue_5 (Math|Vector|MakeVector 1.0 _returnvalue_3 _returnvalue_3) Location _returnvalue_4 2e+01))))

(event EventBeginPlay
  (Utilities|FlowControl|Sequence
    (:then_0
      ;[1 1 1] BloodSplatter
      (bind _returnvalue (Effects|SpawnEmitteratLocation "/Game/ZombiesAndDemons/BloodEffects/Particles/P_BloodSpray_GIBS.P_BloodSpray_GIBS" (Transformation|GetActorLocation) "0, 0, 0" (Variables|/Script/Engine.SceneComponent|GetRelativeScale3D (Variables|Default|GetScene))))
      (EventDispatchers|BindEventtoOnParticleCollide _returnvalue (delegate Custom|CustomEvent)))
    (:then_1
      ;[1 1 1] Blood Trails
      (EventDispatchers|BindEventtoOnParticleCollide (Variables|Default|GetBloodTrails1) (delegate Custom|CustomEvent_5))
      (Utilities|FlowControl|Delay 3.0)
      (Components|Activation|Deactivate (Variables|Default|GetBloodTrails2)))
    (:then_2
      ;[1 1 1] Random impulse to spread the gibs
      (Physics|AddImpulse (Variables|Default|GetMesh1) (Math|Vector|MakeVector (Math|Random|RandomFloatinRange -5e+01 5e+01) (Math|Random|RandomFloatinRange -5e+01 5e+01) (Math|Random|RandomFloatinRange 5e+01 1e+02)) "None" false)
      (Physics|AddImpulse (Variables|Default|GetMesh2) (Math|Vector|MakeVector (Math|Random|RandomFloatinRange -5e+01 5e+01) (Math|Random|RandomFloatinRange -5e+01 5e+01) (Math|Random|RandomFloatinRange 5e+01 1e+02)) "None" false)
      (Physics|AddImpulse (Variables|Default|GetMesh3) (Math|Vector|MakeVector (Math|Random|RandomFloatinRange -5e+01 5e+01) (Math|Random|RandomFloatinRange -5e+01 5e+01) (Math|Random|RandomFloatinRange 5e+01 1e+02)) "None" false)
      (Physics|AddImpulse (Variables|Default|GetMesh4) (Math|Vector|MakeVector (Math|Random|RandomFloatinRange -5e+01 5e+01) (Math|Random|RandomFloatinRange -5e+01 5e+01) (Math|Random|RandomFloatinRange 5e+01 1e+02)) "None" false))
    (:then_4
      (Audio|PlaySoundatLocation "/Game/ZombiesAndDemons/BloodEffects/Sounds/SC_Gibs.SC_Gibs" (Transformation|GetActorLocation) "0, 0, 0" 1.0 1.0 0.0 0 0 0))))

(event Collision|EventHit
  (params (MyComp :type Primitive%20Component%20Object%20Reference) (Other :type Actor%20Object%20Reference) (OtherComp :type Primitive%20Component%20Object%20Reference) (bSelfMoved :type Boolean) (HitLocation :type Vector :default "0, 0, 0") (HitNormal :type Vector :default "0, 0, 0") (NormalImpulse :type Vector :default "0, 0, 0") (Hit :type Hit%20Result%20Structure%20%28by%20ref%29))
  (bind _bloodtrails1 (Variables|Default|GetBloodTrails1))
  (bind _bloodtrails2 (Variables|Default|GetBloodTrails2))
  (bind _bloodtrails3 (Variables|Default|GetBloodTrails3))
  (bind _bloodtrails4 (Variables|Default|GetBloodTrails4))
  ;[1 1 1] Deactivate particle when the gib is not moving
  (Utilities|FlowControl|Sequence
    (:then_0
      (if (Math|Vector|Equal(Vector) (Transformation|GetComponentVelocity (Variables|Default|GetMesh1)) "0, 0, 0" 1e+02) :!label _label
        (if (Components|Activation|IsActive (Variables|Default|GetBloodTrails1))
          (Components|Activation|Deactivate _bloodtrails1))
        (elif (Math|Boolean|NotEqual(Boolean) (Components|Activation|IsActive (Variables|Default|GetBloodTrails1)) true)
          (Components|Activation|Activate _bloodtrails1 false)))
      (Utilities|FlowControl|Delay 0.2)
      (goto _label))
    (:then_1
      (if (Math|Vector|Equal(Vector) (Transformation|GetComponentVelocity (Variables|Default|GetMesh2)) "0, 0, 0" 1e+02) :!label _label_2
        (if (Components|Activation|IsActive (Variables|Default|GetBloodTrails2))
          (Components|Activation|Deactivate _bloodtrails2))
        (elif (Math|Boolean|NotEqual(Boolean) (Components|Activation|IsActive (Variables|Default|GetBloodTrails2)) true)
          (Components|Activation|Activate _bloodtrails2 false)))
      (Utilities|FlowControl|Delay 0.2)
      (goto _label_2))
    (:then_2
      (if (Math|Vector|Equal(Vector) (Transformation|GetComponentVelocity (Variables|Default|GetMesh3)) "0, 0, 0" 1e+02) :!label _label_3
        (if (Components|Activation|IsActive (Variables|Default|GetBloodTrails3))
          (Components|Activation|Deactivate _bloodtrails3))
        (elif (Math|Boolean|NotEqual(Boolean) (Components|Activation|IsActive (Variables|Default|GetBloodTrails3)) true)
          (Components|Activation|Activate _bloodtrails3 false)))
      (Utilities|FlowControl|Delay 0.2)
      (goto _label_3))
    (:then_3
      (if (Math|Vector|Equal(Vector) (Transformation|GetComponentVelocity (Variables|Default|GetMesh4)) "0, 0, 0" 1e+02) :!label _label_4
        (if (Components|Activation|IsActive (Variables|Default|GetBloodTrails4))
          (Components|Activation|Deactivate _bloodtrails4))
        (elif (Math|Boolean|NotEqual(Boolean) (Components|Activation|IsActive (Variables|Default|GetBloodTrails4)) true)
          (Components|Activation|Activate _bloodtrails4 false)))
      (Utilities|FlowControl|Delay 0.2)
      (goto _label_4))))

(fn ConstructionScript)