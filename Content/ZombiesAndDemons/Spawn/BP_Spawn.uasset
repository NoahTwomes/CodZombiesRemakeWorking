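; BP_Spawn is a spawner that produces zombies and demons up to a repeat limit, optionally starting after a timer.
; Flags select alternating types, zombies only or demons only, using a random MultiGate for zombie variants and a chance roll for big demons.
; It picks its own location or a navigable point within a radius, plays a decal and emitter, spawns after a short delay, then re-calls itself.
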(event Custom|Spawn
  (Utilities|FlowControl|DoN (Variables|Default|GetRepeats)
    (:Exit
      (if (Variables|Default|GetRandom)
        (Utilities|FlowControl|FlipFlop
          (:A
            (Utilities|FlowControl|MultiGate true true -1 :!label _label
              (:Out%200
                (Variables|Default|SetActor "/Game/ZombiesAndDemons/Characters/Blueprints/BP_Zombies_Child1.BP_Zombies_Child1_C"))
              (:Out%201
                (Variables|Default|SetActor "/Game/ZombiesAndDemons/Characters/Blueprints/BP_Zombies_Child2.BP_Zombies_Child2_C"))
              (:Out%202
                (Variables|Default|SetActor "/Game/ZombiesAndDemons/Characters/Blueprints/BP_Zombies_Child3.BP_Zombies_Child3_C"))
              (:Out%203
                (Variables|Default|SetActor "/Game/ZombiesAndDemons/Characters/Blueprints/BP_Zombies_Child4.BP_Zombies_Child4_C"))
              (:Out%204
                (Variables|Default|SetActor "/Game/ZombiesAndDemons/Characters/Blueprints/BP_Zombies_Child5.BP_Zombies_Child5_C"))
              (:Out%205
                (Variables|Default|SetActor "/Game/ZombiesAndDemons/Characters/Blueprints/BP_Zombies_Child6.BP_Zombies_Child6_C"))
              (:Out%206
                (Variables|Default|SetActor "/Game/ZombiesAndDemons/Characters/Blueprints/BP_Zombies_Child7.BP_Zombies_Child7_C"))
              (:Out%207
                (Variables|Default|SetActor "/Game/ZombiesAndDemons/Characters/Blueprints/BP_Zombies_Child8.BP_Zombies_Child8_C"))))
          (:B
            (if (== (Math|Random|RandomIntegerinRange 0 (Variables|Default|GetBigDemonChance)) 1) :!label _label_2
              (Variables|Default|SetActor "/Game/ZombiesAndDemons/Characters/Blueprints/BP_Demons_Child_BigDemon.BP_Demons_Child_BigDemon_C")
              (else
                (Variables|Default|SetActor "/Game/ZombiesAndDemons/Characters/Blueprints/BP_Demons.BP_Demons_C")))))
        (if (> (Variables|Default|GetRadius) 0)
          (Variables|Default|SetLocation (.RandomLocation (Class|NavigationSystemV1|GetRandomPointinNavigableRadius (Transformation|GetActorLocation) (Math|Conversions|ToFloat(Integer) (Variables|Default|GetRadius)) 0 0)))
          (else
            (Variables|Default|SetLocation (Transformation|GetActorLocation))))
        (Rendering|Decal|SpawnDecalatLocation "/Game/ZombiesAndDemons/Spawn/Materials/M_Spawn1_Inst1.M_Spawn1_Inst1" "20.000000,100.000000,100.000000" (Variables|Default|GetLocation) "-90.000000,0.000000,0.000000" 1.0)
        (Effects|SpawnEmitteratLocation "/Game/ZombiesAndDemons/Spawn/Particles/P_SpawnDischarge_RED.P_SpawnDischarge_RED" (Variables|Default|GetLocation))
        (Utilities|FlowControl|Delay 0.5)
        (Game|SpawnActorfromClass (Variables|Default|GetActor) (Math|Conversions|ToTransform(Vector) (+ (Variables|Default|GetLocation) "0, 0,100.000000")) "AdjustIfPossibleButAlwaysSpawn" 0 0)
        (Utilities|FlowControl|Delay (Variables|Default|GetLoopDelay))
        (CallFunction|Spawn)
        (elif (Variables|Default|GetZombie)
          (goto _label)
          (elif (Variables|Default|GetDemon)
            (goto _label_2)))))))

(event EventBeginPlay
  (bind _timer (Variables|Default|GetTimer))
  (if (> _timer 0)
    (Utilities|FlowControl|Delay (Math|Conversions|ToFloat(Integer) _timer))
    (CallFunction|Spawn)))

(fn ConstructionScript)