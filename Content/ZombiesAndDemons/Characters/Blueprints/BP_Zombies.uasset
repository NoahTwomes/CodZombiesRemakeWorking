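; Zombie enemy character that optionally roams with periodic moans, chases the first player it senses, and claws at close range.
; Roam and Chase loop on AIMoveTo; reaching the target triggers a two-hit line-trace attack synced to the AnimBP.
; Point damage spawns blood and records the hit body region.
; Lethal damage uses that region to swap in gib meshes, with randomized head variants, blood emitters, detached parts and ragdoll.
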(event OnSeePawn(PawnSensing)
  (params (Pawn :type Pawn%20Object%20Reference))
  ;[1 1 1] OnSeePawn
  (if (and (Pawn|IsPlayerControlled Pawn) (Variables|Default|GetAlive))
    (Utilities|FlowControl|DoOnce false
      (:Completed
        (Variables|Default|SetEnemy Pawn)
        (CallFunction|Chase)
        (bind _returnvalue (Audio|SpawnSoundAttached "/Game/ZombiesAndDemons/Characters/Sounds/SC_Zombie_Awake.SC_Zombie_Awake" (Variables|Character|GetMesh) "None" "0, 0, 0" "0, 0, 0" "KeepRelativeOffset" false 1.0 1.0 0.0 0 0))))))

(event Custom|Chase
  ;[1 1 1] Chase
  (AI|AIMoveTo self "0, 0, 0" (Variables|Default|GetEnemy) 5.0 false
    (:then
      (Utilities|FlowControl|Delay 1.0)
      (CallFunction|Chase))
    (:OnSuccess
      (CallFunction|Attack))))

(event Custom|Roam
  ;[1 1 1] Roam
  (AI|AIMoveTo self (.RandomLocation (AI|Navigation|GetRandomReachablePointinRadius (Transformation|GetActorLocation) 1e+03 0 0)) 0 5.0 false
    (:then
      (Utilities|FlowControl|Delay 1.0)
      (if (not (Utilities|IsValid (Variables|Default|GetEnemy)))
        (CallFunction|Roam)))))

(event Custom|Attack
  ;[1 1 1] Attack
  (CallFunction|Claws))

(event Custom|Death
  ;[1 1 1] Death
  (Variables|Default|SetAlive false)
  (Physics|SetSimulatePhysics (Variables|Character|GetMesh) true)
  (Collision|SetCollisionEnabled (Variables|Collision|GetCapsuleComponent) "NoCollision"))

(event Custom|GIBS
  (bind _returnvalue (Utilities|Name|MakeLiteralName "spine_01"))
  (bind _mesh (Variables|Character|GetMesh))
  (bind _mesh_2 (Variables|Character|GetMesh))
  ;[1 1 1] GIBS_selector
  (Variables|Default|SetAlive false)
  (Utilities|FlowControl|Sequence
    (:then_0
      (switch int (Variables|Default|GetGIBS_selector)
        (:1
          (Utilities|FlowControl|MultiGate true false -1 ; Random Effect For Head hit
            (:Out%200
              (Components|SkinnedMesh|SetSkinnedAssetandUpdate (Variables|Character|GetMesh) (Variables|Default|GetMesh_GIBS_HEAD_neck) false)
              (Effects|SpawnEmitterAttached "/Game/ZombiesAndDemons/BloodEffects/Particles/P_GIBS_Blood.P_GIBS_Blood" (Variables|Character|GetMesh) "GIBS_HEAD_LOWER")
              (Effects|SpawnEmitterAttached "/Game/ZombiesAndDemons/BloodEffects/Particles/P_GIBS_Blood.P_GIBS_Blood" (Variables|Character|GetMesh) "GIBS_HEAD_UPPER"))
            (:Out%201
              (Components|SkinnedMesh|SetSkinnedAssetandUpdate (Variables|Character|GetMesh) (Variables|Default|GetMesh_GIBS_HEAD_half) false)
              (Effects|SpawnEmitterAttached "/Game/ZombiesAndDemons/BloodEffects/Particles/P_GIBS_Blood.P_GIBS_Blood" (Variables|Character|GetMesh) "GIBS_HEAD_LOWER")
              (Utilities|FlowControl|MultiGate true false -1
                (:Out%200
                  (Components|SkinnedMesh|HideBonebyName (Variables|Character|GetMesh) "horn_l" "PBO_None")
                  (Game|SpawnActorfromClass "/Game/ZombiesAndDemons/BloodEffects/BP_Gibs.BP_Gibs_C" (Transformation|GetSocketTransform (Variables|Character|GetMesh) "head" "RTS_World") "Undefined" "OverrideRootScale" 0 0)
                  (Class|SkeletalMeshComponent|SetAllBodiesBelowSimulatePhysics _mesh_2 _returnvalue true true :!label _label)
                  (Class|SkeletalMeshComponent|SetAllBodiesBelowPhysicsBlendWeight _mesh_2 _returnvalue 0.8 false true)
                  (Utilities|FlowControl|Delay 1.0))
                (:Out%201
                  (Effects|SpawnEmitterAttached "/Game/ZombiesAndDemons/BloodEffects/Particles/P_GIBS_Blood.P_GIBS_Blood" (Variables|Character|GetMesh) "GIBS_HEAD_UPPER"))))
            (:Out%202
              (Components|SkinnedMesh|SetSkinnedAssetandUpdate (Variables|Character|GetMesh) (Variables|Default|GetMesh_GIBS_HEAD_L) false)
              (Effects|SpawnEmitterAttached "/Game/ZombiesAndDemons/BloodEffects/Particles/P_GIBS_Blood.P_GIBS_Blood" (Variables|Character|GetMesh) "GIBS_HORN_L_1")
              (Utilities|FlowControl|MultiGate true false -1
                (:Out%200
                  (Components|SkinnedMesh|HideBonebyName (Variables|Character|GetMesh) "horn_l" "PBO_None")
                  (Game|SpawnActorfromClass "/Game/ZombiesAndDemons/BloodEffects/BP_Gibs.BP_Gibs_C" (Transformation|GetSocketTransform (Variables|Character|GetMesh) "horn_l" "RTS_World") "Undefined" "OverrideRootScale" 0 0)
                  (goto _label))
                (:Out%201
                  (Effects|SpawnEmitterAttached "/Game/ZombiesAndDemons/BloodEffects/Particles/P_GIBS_Blood.P_GIBS_Blood" (Variables|Character|GetMesh) "GIBS_HORN_L_2"))))
            (:Out%203
              (Components|SkinnedMesh|SetSkinnedAssetandUpdate (Variables|Character|GetMesh) (Variables|Default|GetMesh_GIBS_HEAD_R) false)
              (Effects|SpawnEmitterAttached "/Game/ZombiesAndDemons/BloodEffects/Particles/P_GIBS_Blood.P_GIBS_Blood" (Variables|Character|GetMesh) "GIBS_HORN_R_1")
              (Utilities|FlowControl|MultiGate true false -1
                (:Out%200
                  (Components|SkinnedMesh|HideBonebyName (Variables|Character|GetMesh) "horn_r" "PBO_None")
                  (Game|SpawnActorfromClass "/Game/ZombiesAndDemons/BloodEffects/BP_Gibs.BP_Gibs_C" (Transformation|GetSocketTransform (Variables|Character|GetMesh) "horn_r" "RTS_World") "Undefined" "OverrideRootScale" 0 0)
                  (goto _label))
                (:Out%201
                  (Effects|SpawnEmitterAttached "/Game/ZombiesAndDemons/BloodEffects/Particles/P_GIBS_Blood.P_GIBS_Blood" (Variables|Character|GetMesh) "GIBS_HORN_R_2"))))
            (:Out%204
              (Components|SkinnedMesh|SetSkinnedAssetandUpdate (Variables|Character|GetMesh) (Variables|Default|GetMesh_GIBS_HEAD) false)
              (Effects|SpawnEmitterAttached "/Game/ZombiesAndDemons/BloodEffects/Particles/P_GIBS_Blood.P_GIBS_Blood" (Variables|Character|GetMesh) "GIBS_HEAD_LOWER")
              (Utilities|FlowControl|MultiGate true false -1
                (:Out%200
                  (Components|SkinnedMesh|HideBonebyName (Variables|Character|GetMesh) "head" "PBO_None")
                  (Game|SpawnActorfromClass "/Game/ZombiesAndDemons/BloodEffects/BP_Gibs.BP_Gibs_C" (Transformation|GetSocketTransform (Variables|Character|GetMesh) "head" "RTS_World") "Undefined" "OverrideRootScale" 0 0)
                  (goto _label))
                (:Out%201
                  (Effects|SpawnEmitterAttached "/Game/ZombiesAndDemons/BloodEffects/Particles/P_GIBS_Blood.P_GIBS_Blood" (Variables|Character|GetMesh) "GIBS_HEAD_UPPER"))))))
        (:2
          (Components|SkinnedMesh|SetSkinnedAssetandUpdate (Variables|Character|GetMesh) (Variables|Default|GetMesh_GIBS_HALF) false)
          (Effects|SpawnEmitterAttached "/Game/ZombiesAndDemons/BloodEffects/Particles/P_GIBS_Blood.P_GIBS_Blood" (Variables|Character|GetMesh) "GIBS_HALF_LOWER")
          (Effects|SpawnEmitterAttached "/Game/ZombiesAndDemons/BloodEffects/Particles/P_GIBS_Blood.P_GIBS_Blood" (Variables|Character|GetMesh) "GIBS_HALF_UPPER"))
        (:3
          (Components|SkinnedMesh|SetSkinnedAssetandUpdate (Variables|Character|GetMesh) (Variables|Default|GetMesh_GIBS_HALF) false)
          (Effects|SpawnEmitterAttached "/Game/ZombiesAndDemons/BloodEffects/Particles/P_GIBS_Blood.P_GIBS_Blood" (Variables|Character|GetMesh) "GIBS_HALF_LOWER")
          (Effects|SpawnEmitterAttached "/Game/ZombiesAndDemons/BloodEffects/Particles/P_GIBS_Blood.P_GIBS_Blood" (Variables|Character|GetMesh) "GIBS_HALF_UPPER"))
        (:4
          (Components|SkinnedMesh|SetSkinnedAssetandUpdate (Variables|Character|GetMesh) (Variables|Default|GetMesh_GIBS_L) false)
          (Effects|SpawnEmitterAttached "/Game/ZombiesAndDemons/BloodEffects/Particles/P_GIBS_Blood.P_GIBS_Blood" (Variables|Character|GetMesh) "GIBS_L_1")
          (Effects|SpawnEmitterAttached "/Game/ZombiesAndDemons/BloodEffects/Particles/P_GIBS_Blood.P_GIBS_Blood" (Variables|Character|GetMesh) "GIBS_L_2"))
        (:5
          (Components|SkinnedMesh|SetSkinnedAssetandUpdate (Variables|Character|GetMesh) (Variables|Default|GetMesh_GIBS_R) false)
          (Effects|SpawnEmitterAttached "/Game/ZombiesAndDemons/BloodEffects/Particles/P_GIBS_Blood.P_GIBS_Blood" (Variables|Character|GetMesh) "GIBS_R_1")
          (Effects|SpawnEmitterAttached "/Game/ZombiesAndDemons/BloodEffects/Particles/P_GIBS_Blood.P_GIBS_Blood" (Variables|Character|GetMesh) "GIBS_R_2")))
      (Physics|SetSimulatePhysics (Variables|Character|GetMesh) true)
      (Collision|SetCollisionEnabled (Variables|Collision|GetCapsuleComponent) "NoCollision"))
    (:then_1
      ;;[1 1 1] SetMaterials
      (Rendering|Material|SetMaterialbyName _mesh "Body" (Variables|Default|GetMat_Body))
      (Rendering|Material|SetMaterialbyName _mesh "GIBS" "/Game/ZombiesAndDemons/Characters/Materials/M_GIBS.M_GIBS")
      (Rendering|Material|SetMaterialbyName _mesh "Skeleton" "/Game/ZombiesAndDemons/Characters/Materials/M_Skeleton.M_Skeleton"))
    (:then_2
      (Variables|/Script/Engine.CharacterMovementComponent|SetMaxWalkSpeed (Variables|Character|GetCharacterMovement) 0.0))))

(event Custom|Claws
  (bind _self self)
  (bind _capsulecomponent (Variables|Collision|GetCapsuleComponent))
  (bind _returnvalue (Transformation|GetWorldLocation _capsulecomponent))
  (bind _returnvalue_2 (Transformation|GetWorldLocation _capsulecomponent))
  (bind _returnvalue_3 (Math|Vector|GetForwardVector _capsulecomponent))
  (bind _returnvalue_4 (* _returnvalue_3 2.5e+02))
  (bind _returnvalue_5 (+ _returnvalue_2 _returnvalue_4))
  ;[1 1 1] Claws
  (if (> (Variables|Default|GetHealth) 0.0)
    (if (or (AI|Components|NavMovement|IsFalling (Variables|Character|GetCharacterMovement)) (> (Transformation|GetDistanceTo (Variables|Default|GetEnemy)) 2.5e+02))
      (Utilities|FlowControl|Delay (Math|Random|RandomFloatinRange 0.5 1.0) :!label _label)
      (else
        (Variables|Default|SetIsAttacking true)
        (Transformation|SetActorRotation _self (Math|Rotator|MakeRotator 0.0 0.0 (.Yaw (Math|Rotator|BreakRotator (Math|Rotator|FindLookatRotation (Transformation|GetActorLocation _self) (Transformation|GetActorLocation (Variables|Default|GetEnemy)))))))
        (Variables|/Script/Engine.CharacterMovementComponent|SetMaxWalkSpeed (Variables|Character|GetCharacterMovement) 0.0)
        (Variables|/Game/ZombiesAndDemons/Characters/Animations/Zombie_AnimBP.Zombie_AnimBP_C|SetIsAttacking (.AsZombie%20Anim%20BP (Utilities|Casting|CastToZombie_AnimBP (Components|SkeletalMesh|GetAnimInstance (Variables|Character|GetMesh)))) true)
        (Utilities|FlowControl|Delay 0.3)
        (if (not (Variables|Default|GetFakeingDeath))
          (Audio|SpawnSoundAttached 0 (Variables|Character|GetMesh) "None" "0, 0, 0" "0, 0, 0" "KeepRelativeOffset" false 1.0 1.0 0.0 0 0)
          (bind _outhit (Collision|LineTraceByChannel _returnvalue _returnvalue_5 "TraceTypeQuery1" false 0 "None"))
          (Game|Damage|ApplyDamage (.HitActor (Collision|BreakHitResult _outhit)) (Variables|Default|GetDamage) 0 (Variables|Actor|GetInstigator))
          (Audio|SpawnSoundatLocation 0 (.Location (Collision|BreakHitResult _outhit)) "0, 0, 0" 1.0 1.0 0.0 0 0)
          (Utilities|FlowControl|Delay 0.3)
          (if (not (Variables|Default|GetFakeingDeath))
            (bind _outhit_2 (Collision|LineTraceByChannel _returnvalue _returnvalue_5 "TraceTypeQuery1" false 0 "None"))
            (Game|Damage|ApplyDamage (.HitActor (Collision|BreakHitResult _outhit_2)) (Variables|Default|GetDamage) 0 (Variables|Actor|GetInstigator))
            (Audio|SpawnSoundatLocation 0 (.Location (Collision|BreakHitResult _outhit_2)) "0, 0, 0" 1.0 1.0 0.0 0 0)
            (Utilities|FlowControl|Delay 0.2)
            (Variables|/Script/Engine.CharacterMovementComponent|SetMaxWalkSpeed (Variables|Character|GetCharacterMovement) (Variables|Default|GetWalkSpeed))
            (Variables|/Game/ZombiesAndDemons/Characters/Animations/Zombie_AnimBP.Zombie_AnimBP_C|SetIsAttacking (.AsZombie%20Anim%20BP (Utilities|Casting|CastToZombie_AnimBP (Components|SkeletalMesh|GetAnimInstance (Variables|Character|GetMesh)))) false)
            (goto _label)))))))

(event EventBeginPlay
  ;[1 1 1] BeginPlay
  (Utilities|FlowControl|Sequence
    (:then_0
      (if (Variables|Default|GetRoamOnStart)
        (CallFunction|Roam)
        ;[1 1 1] ZombieSound
        (Utilities|FlowControl|Delay (Math|Conversions|ToFloat(Integer) (Math|Random|RandomIntegerinRange 5 10)) :!label _label)
        (if (Variables|Default|GetAlive)
          (bind _returnvalue (Audio|SpawnSoundAttached "/Game/ZombiesAndDemons/Characters/Sounds/SC_Zaombie_Moan.SC_Zaombie_Moan" (Variables|Character|GetMesh) "None" "0, 0, 0" "0, 0, 0" "KeepRelativeOffset" false 1.0 1.0 0.0 0 0))
          (goto _label))
        (else
          ;[1 1 1] Walk/Runs Animations Scale
          (Variables|/Game/ZombiesAndDemons/Characters/Animations/Demons_AnimBP.Demons_AnimBP_C|SetScale (.AsDemons%20Anim%20BP (Utilities|Casting|CastToDemons_AnimBP (Components|SkeletalMesh|GetAnimInstance (Variables|Character|GetMesh)))) (.Z (Math|Vector|BreakVector (Transformation|GetWorldScale (Variables|Collision|GetCapsuleComponent))))))))))

(event Game|Damage|EventAnyDamage
  (params (Damage :type Float%20%28single-precision%29) (DamageType :type Damage%20Type%20Object%20Reference) (InstigatedBy :type Controller%20Object%20Reference) (DamageCauser :type Actor%20Object%20Reference))
  ;[1 1 1] AnyDamage
  (if (Variables|Default|GetAlive)
    (Utilities|FlowControl|Sequence
      (:then_0
        ;;[1 1 1] HitSound
        (Utilities|FlowControl|DoOnce false :!label _label
          (:Completed
            (Audio|SpawnSoundAttached "/Game/ZombiesAndDemons/Characters/Sounds/SC_Zombie_Get_Hit.SC_Zombie_Get_Hit" (Variables|Character|GetMesh) "None" "0, 0, 0" "0, 0, 0" "KeepRelativeOffset" false 1.0 1.0 0.0 0 0)
            (Utilities|FlowControl|Delay 0.2)
            (goto _label Reset))))
      (:then_1
        (bind _output_get (Variables|Default|SetHealth (- (Variables|Default|GetHealth) Damage)))
        (if (<= _output_get 0.0)
          (CallFunction|GIBS)
          (Utilities|FlowControl|Sequence
            (:then_0
              (if (Utilities|IsValid (stale EventBeginPlay _returnvalue))
                (Audio|Components|Audio|Stop (stale EventBeginPlay _returnvalue))))
            (:then_1
              (if (Utilities|IsValid (stale OnSeePawn(PawnSensing) _returnvalue))
                (Audio|Components|Audio|Stop (stale OnSeePawn(PawnSensing) _returnvalue))))))))
    (elif (not (Physics|IsSimulatingPhysics (Variables|Character|GetMesh) "pelvis"))
      ;[1 1 1] GIBS_selector
      (Physics|SetSimulatePhysics (Variables|Character|GetMesh) true)
      (Collision|SetCollisionEnabled (Variables|Collision|GetCapsuleComponent) "NoCollision"))))

(event Game|Damage|EventPointDamage
  (params (Damage :type Float%20%28single-precision%29) (DamageType :type Damage%20Type%20Object%20Reference) (HitLocation :type Vector :default "0, 0, 0") (HitNormal :type Vector :default "0, 0, 0") (HitComponent :type Primitive%20Component%20Object%20Reference) (BoneName :type Name :default "None") (ShotFromDirection :type Vector :default "0, 0, 0") (InstigatedBy :type Controller%20Object%20Reference) (DamageCauser :type Actor%20Object%20Reference) (HitInfo :type Hit%20Result%20Structure%20%28by%20ref%29))
  ;[1 1 1] PointDamage
  (Utilities|FlowControl|Sequence
    (:then_0
      (Game|SpawnActorfromClass "/Game/ZombiesAndDemons/BloodEffects/BP_BloodSplatters.BP_BloodSplatters_C" (Math|Transform|MakeTransform HitLocation (Math|Conversions|RotationFromXVector HitNormal)) "Undefined" "OverrideRootScale" 0 0) ; BLOOD
    )
    (:then_1
      (if (Variables|Default|GetAlive)
        ;;[1 1 1] Set gibs effect based on the hit bone
        (if (Utilities|Name|Equal(Name) BoneName "head")
          (Variables|Default|SetGIBS_selector 1)
          (else
            (for _array_element (Variables|Default|GetBones_Half_Upper)
              (if (Utilities|Name|Equal(Name) BoneName _array_element)
                (Variables|Default|SetGIBS_selector 2)))
            (for _array_element_2 (Variables|Default|GetBones_Half_Lower)
              (if (Utilities|Name|Equal(Name) BoneName _array_element_2)
                (Variables|Default|SetGIBS_selector 3)))
            (for _array_element_3 (Variables|Default|GetBones_L)
              (if (Utilities|Name|Equal(Name) BoneName _array_element_3)
                (Variables|Default|SetGIBS_selector 4)))
            (for _array_element_4 (Variables|Default|GetBones_R)
              (if (Utilities|Name|Equal(Name) BoneName _array_element_4)
                (Variables|Default|SetGIBS_selector 5)))))))))

(fn ConstructionScript
  (Variables|/Script/Engine.CharacterMovementComponent|SetMaxWalkSpeed (Variables|Character|GetCharacterMovement) (Variables|Default|GetWalkSpeed))
  (Rendering|Material|SetMaterialbyName (Variables|Character|GetMesh) "Body" (Variables|Default|GetMat_Body)))