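; Green fireball projectile that damages what it hits and explodes.
; On spawn it attaches cast and spark sounds to its Sphere, which ignores the instigator when moving.
; On hit it spawns a green explosion, applies fixed damage with the instigator as causer, and pushes physics-simulating components along its velocity.
; It then destroys itself, with the explosion sound played at the impact point from a later sequence branch.
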(event EventBeginPlay
  ;[1 1 1] OnBeginPlay
  (Utilities|FlowControl|Sequence
    (:then_0
      (Audio|SpawnSoundAttached "/Game/ZombiesAndDemons/Characters/Fireballs/Sounds/SC_Fireball_Cast.SC_Fireball_Cast" (Variables|Default|GetSphere) "None" "0, 0, 0" "0, 0, 0" "KeepRelativeOffset" true 1.0 1.0 0.0 0 0)
      (Audio|SpawnSoundAttached "/Game/ZombiesAndDemons/Characters/Fireballs/Sounds/SC_Fire_Sparks.SC_Fire_Sparks" (Variables|Default|GetSphere) "None" "0, 0, 0" "0, 0, 0" "KeepRelativeOffset" true 1.0 1.0 0.0 0 0))
    (:then_1
      (Collision|IgnoreActorwhenMoving (Variables|Default|GetSphere) (Game|GetInstigator) true))))

(event Collision|EventHit
  (params (MyComp :type Primitive%20Component%20Object%20Reference) (Other :type Actor%20Object%20Reference) (OtherComp :type Primitive%20Component%20Object%20Reference) (bSelfMoved :type Boolean) (HitLocation :type Vector :default "0, 0, 0") (HitNormal :type Vector :default "0, 0, 0") (NormalImpulse :type Vector :default "0, 0, 0") (Hit :type Hit%20Result%20Structure%20%28by%20ref%29))
  ;[1 1 1] OnHit
  (Utilities|FlowControl|Sequence
    (:then_0
      (Effects|SpawnEmitteratLocation "/Game/ZombiesAndDemons/Characters/Fireballs/Particles/P_FireBallExplosion_green.P_FireBallExplosion_green" HitLocation)
      (Game|Damage|ApplyDamage Other 2e+01 0 (Variables|Actor|GetInstigator))
      (if (Utilities|IsValid OtherComp)
        (if (Physics|IsSimulatingPhysics OtherComp "None")
          (Physics|AddImpulseatLocation OtherComp (* (Transformation|GetVelocity) 1e+02) (Transformation|GetActorLocation) (.HitBoneName (Collision|BreakHitResult Hit)))))
      (Actor|DestroyActor) ; Then destroy this projectile
    )
    (:then_2
      (Audio|PlaySoundatLocation "/Game/ZombiesAndDemons/Characters/Fireballs/Sounds/SC_Fireball_Explosion.SC_Fireball_Explosion" HitLocation "0, 0, 0" 1.0 1.0 0.0 0 0 0))))

(fn ConstructionScript)